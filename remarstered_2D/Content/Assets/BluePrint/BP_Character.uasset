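; Player-controlled 2D flipbook character for side-scrolling platforming.
; On BeginPlay it adds the platforming Enhanced Input context, whose actions drive jumping and movement along the X axis, turning the controller yaw to face the input direction.
; Every Tick, UpdateAnimation picks idle or run on the ground by speed; airborne, it shows the Jump flipbook below a vertical velocity threshold and Fall otherwise.
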(event `self.ReceiveBeginPlay`
  (bind _asplayer_controller (cast `PlayerController` (`self.GetController`)))
  (`EnhancedInputSubsystemInterface.AddMappingContext` (pcsubsystem `EnhancedInputLocalPlayerSubsystem` _asplayer_controller) "/Game/Assets/Inputs/IMC_Platforming.IMC_Platforming" 0 (struct)))

(event `EnhancedInput|/Game/Assets/Inputs/Action/IA_Jump`
  (params (ActionValue :type Boolean) (ElapsedSeconds :type "Float (double-precision)") (TriggeredSeconds :type "Float (double-precision)") (InputAction :type "InputAction Object Reference" :default "/Game/Assets/Inputs/Action/IA_Jump.IA_Jump"))
  (:`Started`
    (`self.Jump`))
  (:`Completed`
    (`self.StopJumping`)))

(event `self.ReceiveTick`
  (params (DeltaSeconds :type "Float (single-precision)"))
  (`self.UpdateAnimation`))

(event `EnhancedInput|/Game/Assets/Inputs/Action/IA_Movement`
  (params (ActionValue :type "Float (double-precision)") (ElapsedSeconds :type "Float (double-precision)") (TriggeredSeconds :type "Float (double-precision)") (InputAction :type "InputAction Object Reference" :default "/Game/Assets/Inputs/Action/IA_Movement.IA_Movement"))
  (:`Triggered`
    (`self.AddMovementInput` (1.0 0.0 0.0) ActionValue)
    (`Controller.SetControlRotation` (`self.GetController`) (select `bool` (> ActionValue 0.0) :`false` (`KismetMathLibrary.MakeRotator` 0.0 0.0 180.0) :`true` (`KismetMathLibrary.MakeRotator` 0.0)))))

(fn `UpdateAnimation`
  (bind (_returnvalue_x _returnvalue_y _returnvalue_z) (`KismetMathLibrary.BreakVector` (`self.GetVelocity`)))
  (if (`NavMovementComponent.IsMovingOnGround` (`self.CharacterMovement`))
    (if (> (`KismetMathLibrary.VSize` (`self.GetVelocity`)) 0.0)
      (`PaperFlipbookComponent.SetFlipbook` (`self.Sprite`) "/Game/Assets/Character/FlipBook/FB_Character_run.FB_Character_run")
      (else
        (`PaperFlipbookComponent.SetFlipbook` (`self.Sprite`) "/Game/Assets/Character/FlipBook/FB_Character_Idle.FB_Character_Idle")))
    (elif (< _returnvalue_z 100.0)
      (`PaperFlipbookComponent.SetFlipbook` (`self.Sprite`) "/Game/Assets/Character/FlipBook/FB_Character_Jump.FB_Character_Jump")
      (else
        (`PaperFlipbookComponent.SetFlipbook` (`self.Sprite`) "/Game/Assets/Character/FlipBook/FB_Character_Fall.FB_Character_Fall")))))

(fn `UserConstructionScript`)